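; Zombie NPC actor Blueprint that loses health on capsule overlaps and shows it on a widget health bar.
; Each overlap, from any actor, subtracts a fixed amount until Health is below one.
; A further overlap then activates a particle system, plays a collapse sound and hides the mesh and widget without destroying the actor.
; Tick casts the widget to NPC and updates its progress bar from Health every frame.
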(event OnComponentBeginOverlap(Capsule)
  (params (OverlappedComponent :type Primitive%20Component%20Object%20Reference) (OtherActor :type Actor%20Object%20Reference) (OtherComp :type Primitive%20Component%20Object%20Reference) (OtherBodyIndex :type Integer) (bFromSweep :type Boolean) (SweepResult :type Hit%20Result%20Structure%20%28by%20ref%29))
  (CallFunction|NPCHealthEvent))

(event EventBeginPlay)

(event Collision|EventActorBeginOverlap
  (params (OtherActor :type Actor%20Object%20Reference)))

(event EventTick
  (params (DeltaSeconds :type Float%20%28single-precision%29))
  (CallFunction|NPCGetHealth))

(fn ConstructionScript)

(fn NPCHealthEvent
  (if (< (Variables|Default|GetHealth) 1.0)
    (Components|Activation|Activate (Variables|Default|GetParticleSystem) false)
    (Rendering|SetVisibility (Variables|SkeletalMeshActor|GetSkeletalMeshComponent) false false)
    (Rendering|SetVisibility (Variables|Default|GetWidget) false false)
    (Audio|PlaySoundatLocation "/Game/StarterContent/Audio/Collapse02.Collapse02" (Transformation|GetActorLocation))
    (else
      (Variables|Default|SetHealth (- (Variables|Default|GetHealth) 1e+01)))))

(fn NPCGetHealth
  (bind _asnpc (Utilities|Casting|CastToNPC (UserInterface|GetUserWidgetObject (Variables|Default|GetWidget))))
  (Progress|SetPercent (Variables|/Game/UI/NPC.NPC_C|GetProgressBar_0 _asnpc) (/ (Variables|Default|GetHealth) 1e+02)))